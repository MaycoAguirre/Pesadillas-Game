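; BP_ENEMIGO is an enemy actor that moves along a configurable path and dies when its health runs out.
; The construction script gives InterpToMovement two relative control points, the origin and Pos.
; Projectile hits arrive through the BPIProyectil interface and feed RecibirDaño, which reduces VidaActual and destroys the actor at zero or below.
; PawnSensing stores the seen pawn and only prints an attack message, with no attack implemented.
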(event `self.ReceiveBeginPlay`
  (set `self.VidaActual` (`self.VidaMax`)))

(event `/Game/Blueprints/Interfaces/BPI_DañoProyectil.BPI_Proyectil`
  (params (`DañoProyectil` :type "Float (double-precision)"))
  (`self.RecibirDaño` `DañoProyectil`))

(event `self.PawnSensing.OnSeePawn`
  (params (Pawn :type "Pawn Object Reference"))
  (bind _output_get (set `self.Pawn` Pawn))
  (`KismetSystemLibrary.PrintString` (`KismetStringLibrary.Concat_StrStr` "Atacaria a " (`KismetSystemLibrary.GetDisplayName` _output_get))))

(fn `RecibirDaño`
  (params (`DañoRecibido` :type "Float (double-precision)"))
  (bind _output_get (set `self.VidaActual` (- (`self.VidaActual`) `DañoRecibido`)))
  (if (<= _output_get 0.0)
    (`self.K2_DestroyActor`)))

(fn `UserConstructionScript`
  (`InterpToMovementComponent.AddControlPointPosition` (`self.InterpToMovement`) (0.0 0.0 0.0) true)
  (`InterpToMovementComponent.AddControlPointPosition` (`self.InterpToMovement`) (`self.Pos`) true))